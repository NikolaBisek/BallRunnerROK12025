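; Player-controlled ball that rolls and jumps through physics on its Sphere component.
; Forward/back and left/right axis inputs share one acceleration-based torque call, scaled by BallSpeed on X (negated) and Y.
; Jump press applies an upward velocity-change impulse of Jumpheight through a DoOnce, which resets after a short delay following button release to prevent repeated jumps.
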(event Input|ActionEvents|InputActionJump
  (params (Key :type Key%20Structure :default "None"))
  (:Pressed
    (Utilities|FlowControl|DoOnce false :!label _label
      (:Completed
        (Physics|AddImpulse (Variables|Default|GetSphere) (Math|Vector|MakeVector 0.0 0.0 (Variables|Default|GetJumpheight)) "None" true))))
  (:Released
    (Utilities|FlowControl|Delay 1.2)
    (goto _label Reset)))

(event Input|AxisEvents|InputAxisForwardbackward
  (params (AxisValue :type Float%20%28single-precision%29))
  (bind _ball_speed (Variables|Default|GetBall%20speed))
  (Class|PrimitiveComponent|AddTorqueinRadians (Variables|Default|GetSphere) (Math|Vector|MakeVector (* (* (stale Input|AxisEvents|InputAxisLeftright AxisValue) _ball_speed) -1.0) (* AxisValue _ball_speed) 0.0) "None" true))

(event Input|AxisEvents|InputAxisLeftright
  (params (AxisValue :type Float%20%28single-precision%29))
  (bind _ball_speed (Variables|Default|GetBall%20speed))
  (Class|PrimitiveComponent|AddTorqueinRadians (Variables|Default|GetSphere) (Math|Vector|MakeVector (* (* AxisValue _ball_speed) -1.0) (* (stale Input|AxisEvents|InputAxisForwardbackward AxisValue) _ball_speed) 0.0) "None" true))

(fn ConstructionScript)