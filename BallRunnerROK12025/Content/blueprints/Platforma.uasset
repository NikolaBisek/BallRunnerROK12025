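; Platforma is a platform that tilts when the player's Ball_BP pawn enters its Box trigger.
; Begin overlap sets a tilting flag only for that ball, while any end overlap clears it.
; Each Tick, FInterpTo eases the Cube's relative roll toward Tiltangle while flagged, or back to zero otherwise, at Tiltspeed with scaled-down delta time, keeping pitch and yaw at zero.
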(event OnComponentBeginOverlap(Box)
  (params (OverlappedComponent :type Primitive%20Component%20Object%20Reference) (OtherActor :type Actor%20Object%20Reference) (OtherComp :type Primitive%20Component%20Object%20Reference) (OtherBodyIndex :type Integer) (bFromSweep :type Boolean) (SweepResult :type Hit%20Result%20Structure%20%28by%20ref%29))
  (bind _asball_bp (Utilities|Casting|CastToBall_BP (Game|Player|GetPlayerPawn 0)))
  (if (== OtherActor _asball_bp)
    (Variables|Default|Setistilting true)))

(event OnComponentEndOverlap(Box)
  (params (OverlappedComponent :type Primitive%20Component%20Object%20Reference) (OtherActor :type Actor%20Object%20Reference) (OtherComp :type Primitive%20Component%20Object%20Reference) (OtherBodyIndex :type Integer))
  (Variables|Default|Setistilting false))

(event EventTick
  (params (DeltaSeconds :type Float%20%28single-precision%29))
  (bind _returnvalue (* DeltaSeconds 0.1))
  (bind _tiltspeed (Variables|Default|Gettiltspeed))
  (bind _cube (Variables|Default|GetCube))
  (bind _cube_2 (Variables|Default|GetCube))
  (bind _relativerotation (Variables|/Script/Engine.SceneComponent|GetRelativeRotation _cube))
  (if (Variables|Default|Getistilting)
    (Transformation|SetRelativeRotation _cube_2 (Math|Rotator|MakeRotator (Math|Interpolation|FInterpTo (.roll _relativerotation) (Variables|Default|Gettiltangle) _returnvalue _tiltspeed) 0.0 0.0) false false)
    (else
      (Transformation|SetRelativeRotation _cube_2 (Math|Rotator|MakeRotator (Math|Interpolation|FInterpTo (.roll _relativerotation) 0.0 _returnvalue _tiltspeed) 0.0 0.0) false false))))

(fn ConstructionScript)